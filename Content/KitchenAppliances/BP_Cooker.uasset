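; BP_Cooker is a kitchen cooker actor that snaps frying pans onto its four burners.
; Each burner's begin-overlap feeds a shared OnBurnerOverlap event, which prints a debug string, then continues only for BP_FryingPan actors.
; It zeroes the pan mesh's velocities and moves it to the burner's location upright, keeping yaw and scale.
; The burner's overlap events are switched off during the move and restored afterwards.
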(event OnComponentBeginOverlap(BottomLeftBurner)
  (params (OverlappedComponent :type Primitive%20Component%20Object%20Reference) (OtherActor :type Actor%20Object%20Reference) (OtherComp :type Primitive%20Component%20Object%20Reference) (OtherBodyIndex :type Integer) (bFromSweep :type Boolean) (SweepResult :type Hit%20Result%20Structure%20%28by%20ref%29))
  (CallFunction|OnBurnerOverlap OverlappedComponent OtherActor))

(event OnComponentBeginOverlap(BottomRightBurner)
  (params (OverlappedComponent :type Primitive%20Component%20Object%20Reference) (OtherActor :type Actor%20Object%20Reference) (OtherComp :type Primitive%20Component%20Object%20Reference) (OtherBodyIndex :type Integer) (bFromSweep :type Boolean) (SweepResult :type Hit%20Result%20Structure%20%28by%20ref%29))
  (CallFunction|OnBurnerOverlap OverlappedComponent OtherActor))

(event OnComponentBeginOverlap(TopLeftBurner)
  (params (OverlappedComponent :type Primitive%20Component%20Object%20Reference) (OtherActor :type Actor%20Object%20Reference) (OtherComp :type Primitive%20Component%20Object%20Reference) (OtherBodyIndex :type Integer) (bFromSweep :type Boolean) (SweepResult :type Hit%20Result%20Structure%20%28by%20ref%29))
  (CallFunction|OnBurnerOverlap OverlappedComponent OtherActor))

(event OnComponentBeginOverlap(TopRightBurner)
  (params (OverlappedComponent :type Primitive%20Component%20Object%20Reference) (OtherActor :type Actor%20Object%20Reference) (OtherComp :type Primitive%20Component%20Object%20Reference) (OtherBodyIndex :type Integer) (bFromSweep :type Boolean) (SweepResult :type Hit%20Result%20Structure%20%28by%20ref%29))
  (CallFunction|OnBurnerOverlap OverlappedComponent OtherActor))

(event Custom|On%20Burner%20Overlap
  (params (OverlappedComponent :type Primitive%20Component%20Object%20Reference) (OtherActor :type Actor%20Object%20Reference))
  (Development|PrintString "Hello")
  (bind _asbp_frying_pan (Utilities|Casting|CastToBP_FryingPan OtherActor))
  (Variables|/Script/Engine.PrimitiveComponent|SetbGenerateOverlapEvents OverlappedComponent false)
  (Physics|SetPhysicsLinearVelocity (Variables|/Game/Kitchenware/BP_FryingPan.BP_FryingPan_C|GetMesh _asbp_frying_pan) "0, 0, 0" false "None")
  (Class|PrimitiveComponent|SetPhysicsAngularVelocityinRadians (Variables|/Game/Kitchenware/BP_FryingPan.BP_FryingPan_C|GetMesh _asbp_frying_pan) "0, 0, 0" false "None")
  (Transformation|SetActorTransform _asbp_frying_pan (Math|Transform|MakeTransform (Transformation|GetWorldLocation OverlappedComponent) (Math|Rotator|MakeRotator 0.0 0.0 (.Yaw (Math|Rotator|BreakRotator (Transformation|GetActorRotation _asbp_frying_pan)))) (Transformation|GetActorScale3D _asbp_frying_pan)))
  (Variables|/Script/Engine.PrimitiveComponent|SetbGenerateOverlapEvents OverlappedComponent true))

(event EventBeginPlay)

(event Collision|EventActorBeginOverlap
  (params (OtherActor :type Actor%20Object%20Reference)))

(event EventTick
  (params (DeltaSeconds :type Float%20%28single-precision%29)))

(fn ConstructionScript)