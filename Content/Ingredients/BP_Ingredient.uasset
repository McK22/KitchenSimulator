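; BP_Ingredient is a cookable ingredient Blueprint that shows its cooking progress on its mesh.
; On BeginPlay it creates a dynamic material instance for the mesh's first material slot.
; Its Cook override runs the parent logic, then sets the CookingProgress material parameter to cooking time as a fraction of the maximum.
; The construction script applies the current State through SetState.
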(event EventBeginPlay
  ;[1 1 1] Create dynamic material instance for handling cooking
  (bind _returnvalue (Rendering|Material|CreateDynamicMaterialInstance (Variables|Character|GetMesh) 0 0 "None" :!class /Script/Engine.PrimitiveComponent))
  (Variables|Default|SetDynamicMaterialInstance _returnvalue))

(event Collision|EventActorBeginOverlap
  (params (OtherActor :type Actor%20Object%20Reference)))

(event EventTick
  (params (DeltaSeconds :type Float%20%28single-precision%29)))

(event EventCook
  (params (DeltaTime :type Float%20%28single-precision%29))
  ;[1 1 1] Update mesh material after cooking update
  (|CallParentFunction DeltaTime)
  (Rendering|Material|SetScalarParameterValue (Variables|Default|GetDynamicMaterialInstance) "CookingProgress" (/ (Variables|Default|GetCookingTime) (Variables|Default|GetMaxCookingTime)) :!class /Script/Engine.MaterialInstanceDynamic))

(fn ConstructionScript
  (Class|Ingredient|SetState (Variables|Default|GetState)))